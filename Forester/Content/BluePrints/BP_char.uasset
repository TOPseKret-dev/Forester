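; BP_char is a player character Blueprint with movement and basic tree and stone harvesting.
; Two input axes drive movement along the actor's forward and right vectors.
; Attack damages the first HarvestTree entry only while UsingAxe is set.
; The object action damages the first HarvestStone entry and increments CountStone; this graph only reads both target arrays and never fills them.
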(event `InputAxis|F_Move`
  (params (AxisValue :type "Float (single-precision)"))
  (`self.AddMovementInput` (`self.GetActorForwardVector`) AxisValue))

(event `InputAxis|R_Move`
  (params (AxisValue :type "Float (single-precision)"))
  (`self.AddMovementInput` (`self.GetActorRightVector`) AxisValue))

(event `InputAction|Attack`
  (params (Key :type "Key Structure"))
  (bind _output (`|GetArrayItem` (`self.Harvest Tree`)))
  (:`Pressed`
    (if (`self.UsingAxe`)
      (`/Engine/EditorBlueprintResources/StandardMacros.IsValid` _output
        (:`Is Valid`
          (`GameplayStatics.ApplyDamage` _output 25.0 null self))))))

(event `InputAction|ActionWIthObject`
  (params (Key :type "Key Structure"))
  (bind _output (`|GetArrayItem` (`self.Harvest Stone`)))
  (:`Pressed`
    (`/Engine/EditorBlueprintResources/StandardMacros.IsValid` _output
      (:`Is Valid`
        (`GameplayStatics.ApplyDamage` _output 1.0 null self)
        (set `self.CountStone` (+ (`self.CountStone`) 1))))))

(fn `UserConstructionScript`)