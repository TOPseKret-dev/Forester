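; Behavior tree service that stores the location of a BP_char actor in a blackboard vector key for AI use.
; On activation it finds all BP_char actors and writes the first one's location to the configured key, with no tick update or empty-array check.
; Debug prints show the location before the write and the blackboard value after it.
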(event `self.ReceiveActivationAI`
  (params (OwnerController :type "AIController Object Reference") (ControlledPawn :type "Pawn Object Reference"))
  (bind _outactors (`GameplayStatics.GetAllActorsOfClass` "/Game/BluePrints/BP_char.BP_char_C"))
  (bind _returnvalue (`Actor.K2_GetActorLocation` (`|GetArrayItem` _outactors)))
  (`KismetSystemLibrary.PrintString` (`KismetStringLibrary.Conv_VectorToString` _returnvalue) true true (struct :`G` 0.66 :`B` 1.0 :`A` 1.0) 0.0)
  (`BTFunctionLibrary.SetBlackboardValueAsVector` (`self.Blackboard Key`) _returnvalue)
  (`KismetSystemLibrary.PrintString` (`KismetStringLibrary.Conv_VectorToString` (`BTFunctionLibrary.GetBlackboardValueAsVector` (`self.Blackboard Key`))) true true (struct :`G` 0.66 :`B` 1.0 :`A` 1.0) 0.0))