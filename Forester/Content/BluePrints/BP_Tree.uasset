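; BP_Tree is a harvestable tree actor that grants wood and stick resources to the player character when destroyed.
; Its box overlap adds and removes the tree from the player's HarvestTree list while BP_char stands in range.
; Only damage caused by player 0 lowers its health; at zero it destroys itself and increments the player's wood and stick counters.
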(event `self.ReceiveBeginPlay`
  (bind _asbp_char (cast `/Game/BluePrints/BP_char` (`GameplayStatics.GetPlayerCharacter` 0))
    (:`then`
      (set `self.Player` _asbp_char))
    (:`CastFailed`
      _))
  (set `self.Tree Health` (`self.Max Health`)))

(event `self.ReceiveAnyDamage`
  (params (Damage :type "Float (single-precision)") (DamageType :type "DamageType Object Reference") (InstigatedBy :type "Controller Object Reference") (DamageCauser :type "Actor Object Reference"))
  (bind _player (`self.Player`))
  (bind _player_2 (`self.Player`))
  (bind _returnvalue (- (`self.Tree Health`) Damage))
  (if (== DamageCauser (`GameplayStatics.GetPlayerCharacter` 0))
    (if (<= _returnvalue 0.0)
      (bind _output_get (set `self.Tree Health` 0.0))
      (if (== _output_get 0.0)
        (`self.K2_DestroyActor`)
        (set `/Game/BluePrints/BP_char.CountWood` (+ (`/Game/BluePrints/BP_char.CountWood` _player) 2) _player)
        (set `/Game/BluePrints/BP_char.CountStick` (+ (`/Game/BluePrints/BP_char.CountStick` _player_2) 3) _player_2))
      (else
        (set `self.Tree Health` _returnvalue)))))

(event `self.Box.OnComponentBeginOverlap`
  (params (OverlappedComponent :type "PrimitiveComponent Object Reference") (OtherActor :type "Actor Object Reference") (OtherComp :type "PrimitiveComponent Object Reference") (OtherBodyIndex :type Integer) (bFromSweep :type Boolean) (SweepResult :type "HitResult Structure (by ref)"))
  (`/Engine/EditorBlueprintResources/StandardMacros.IsValid` (`self.Player`)
    (:`Is Valid`
      (if (== OtherActor (`self.Player`))
        (`KismetArrayLibrary.Array_Add` (`/Game/BluePrints/BP_char.Harvest Tree` (`self.Player`)) self)))))

(event `self.Box.OnComponentEndOverlap`
  (params (OverlappedComponent :type "PrimitiveComponent Object Reference") (OtherActor :type "Actor Object Reference") (OtherComp :type "PrimitiveComponent Object Reference") (OtherBodyIndex :type Integer))
  (`/Engine/EditorBlueprintResources/StandardMacros.IsValid` (`self.Player`)
    (:`Is Valid`
      (if (== OtherActor (`self.Player`))
        (`KismetArrayLibrary.Array_RemoveItem` (`/Game/BluePrints/BP_char.Harvest Tree` (`self.Player`)) self)))))

(fn `UserConstructionScript`)