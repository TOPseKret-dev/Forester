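; BP_SpawnTreeAndStone is a scatter spawner that populates a box volume with trees and stones when play begins.
; On BeginPlay it runs two loops that spawn CountTree BP_Tree and CountStone BP_Stone actors.
; Each lands at a random point anywhere inside the Box bounds, with random yaw and unit scale.
; Points are used as-is, with no ground trace or spacing check.
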(event `self.ReceiveBeginPlay`
  (bind _box (`self.Box`))
  (bind _box_2 (`self.Box`))
  (for _ (range (`self.Count tree`))
    (`|SpawnActorFromClass` "/Game/BluePrints/BP_Tree.BP_Tree_C" (`KismetMathLibrary.MakeTransform` (`KismetMathLibrary.RandomPointInBoundingBox` (`SceneComponent.K2_GetComponentLocation` _box_2) (`BoxComponent.GetScaledBoxExtent` _box_2)) (`KismetMathLibrary.MakeRotator` 0.0 0.0 (`KismetMathLibrary.Conv_IntToDouble` (`KismetMathLibrary.RandomIntegerInRange` 0 359)))) "Undefined" "OverrideRootScale" null null))
  (for _ (range (`self.Count stone`))
    (`|SpawnActorFromClass` "/Game/BluePrints/BP_Stone.BP_Stone_C" (`KismetMathLibrary.MakeTransform` (`KismetMathLibrary.RandomPointInBoundingBox` (`SceneComponent.K2_GetComponentLocation` _box) (`BoxComponent.GetScaledBoxExtent` _box)) (`KismetMathLibrary.MakeRotator` 0.0 0.0 (`KismetMathLibrary.Conv_IntToDouble` (`KismetMathLibrary.RandomIntegerInRange` 0 359)))) "Undefined" "OverrideRootScale" null null)))

(fn `UserConstructionScript`)