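; AI controller for an enemy that endlessly chases the player character.
; On BeginPlay it caches the first BP_char in the level as its target and starts a self-repeating Move event built on AIMoveTo.
; On success it snaps the pawn's rotation to face the target, and after either success or failure it retries following a short delay.
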(event `self.ReceiveBeginPlay`
  (bind _outactors (`GameplayStatics.GetAllActorsOfClass` "/Game/BluePrints/Charecteres/BP_char.BP_char_C"))
  (set `self.Player` (`|GetArrayItem` _outactors))
  (`self.Move`))

(event `Move`
  (bind _returnvalue (`self.K2_GetPawn`))
  (`|AIMoveTo` (`self.K2_GetPawn`) (0.0 0.0 0.0) (`self.Player`) 75.0
    (:`OnSuccess`
      (`self.K2_SetActorRotation` _returnvalue (`KismetMathLibrary.FindLookAtRotation` (`self.K2_GetActorLocation` _returnvalue) (`self.K2_GetActorLocation` (`self.Player`))) false)
      (`KismetSystemLibrary.Delay` 0.1)
      (`self.Move`))
    (:`OnFail`
      (`KismetSystemLibrary.Delay` 0.1)
      (`self.Move`))))

(fn `UserConstructionScript`)